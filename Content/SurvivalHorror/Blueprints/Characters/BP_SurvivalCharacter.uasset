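; Player character for a survival horror game, handling Enhanced Input movement, camera, crouch, flashlight, interaction, pistol combat and pausing.
; Aiming slows movement, turns the body with the camera, zooms FOV by timeline and holds the shoot montage near-frozen as a pose.
; Camera traces drive interaction and hitscan damage, while ammo and health changes fire notify calls.
; Death ragdolls the mesh and shows the game-over screen.
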(event `self.ReceiveBeginPlay`
  (bind _asplayer_controller (cast `PlayerController` (`self.GetController`)))
  (`EnhancedInputSubsystemInterface.AddMappingContext` (pcsubsystem `EnhancedInputLocalPlayerSubsystem` _asplayer_controller) "/Game/SurvivalHorror/Input/IMC_Survival.IMC_Survival" 0 (struct))
  (bind _returnvalue (`|CreateWidget` "/Game/SurvivalHorror/UI/WBP_HUD.WBP_HUD_C" (`GameplayStatics.GetPlayerController` 0)))
  (`UserWidget.AddToViewport` _returnvalue 0))

(event `EnhancedInput|/Game/SurvivalHorror/Input/Actions/IA_Look`
  (params (ActionValue :type "Vector2D Structure") (ElapsedSeconds :type "Float (double-precision)") (TriggeredSeconds :type "Float (double-precision)") (InputAction :type "InputAction Object Reference" :default "/Game/SurvivalHorror/Input/Actions/IA_Look.IA_Look"))
  (:`Triggered`
    (`self.AddControllerPitchInput` ActionValue_Y)
    (`self.AddControllerYawInput` (* ActionValue_X -1.0))))

(event `EnhancedInput|/Game/SurvivalHorror/Input/Actions/IA_Move`
  (params (ActionValue :type "Vector2D Structure") (ElapsedSeconds :type "Float (double-precision)") (TriggeredSeconds :type "Float (double-precision)") (InputAction :type "InputAction Object Reference" :default "/Game/SurvivalHorror/Input/Actions/IA_Move.IA_Move"))
  (bind _returnvalue (`KismetMathLibrary.MakeRotator` 0.0 0.0 (.yaw (`self.GetControlRotation`))))
  (:`Triggered`
    (`self.AddMovementInput` (`KismetMathLibrary.GetForwardVector` _returnvalue) ActionValue_Y)
    (`self.AddMovementInput` (`KismetMathLibrary.GetRightVector` _returnvalue) ActionValue_X)))

(event `EnhancedInput|/Game/SurvivalHorror/Input/Actions/IA_Aim`
  (params (ActionValue :type Boolean) (ElapsedSeconds :type "Float (double-precision)") (TriggeredSeconds :type "Float (double-precision)") (InputAction :type "InputAction Object Reference" :default "/Game/SurvivalHorror/Input/Actions/IA_Aim.IA_Aim"))
  (bind _charactermovement (`self.CharacterMovement`))
  (bind _charactermovement_2 (`self.CharacterMovement`))
  (:`Started`
    (set `self.bIsAiming` true)
    (set `self.bUseControllerRotationYaw` true)
    (set `CharacterMovementComponent.MaxWalkSpeed` 250.0 _charactermovement_2)
    (set `CharacterMovementComponent.bOrientRotationToMovement` false _charactermovement)
    (`self.PlayAnimMontage` "/Game/SurvivalHorror/Blueprints/Characters/AM_Pistol_Shoot.AM_Pistol_Shoot" 0.0001)
    (bind (_direction _alpha) (`Timeline|TL_Aim` :!label _label)
      (:`Update`
        (`CameraComponent.SetFieldOfView` (`self.FollowCamera`) (`KismetMathLibrary.Lerp` 90.0 65.0 _alpha)))))
  (:`Completed`
    (set `self.bIsAiming` false)
    (set `self.bUseControllerRotationYaw` false)
    (set `CharacterMovementComponent.MaxWalkSpeed` 600.0 _charactermovement)
    (set `CharacterMovementComponent.bOrientRotationToMovement` true _charactermovement_2)
    (`self.StopAnimMontage` "/Game/SurvivalHorror/Blueprints/Characters/AM_Pistol_Shoot.AM_Pistol_Shoot")
    (goto _label :!via `Reverse`)))

(event `EnhancedInput|/Game/SurvivalHorror/Input/Actions/IA_Interact`
  (params (ActionValue :type Boolean) (ElapsedSeconds :type "Float (double-precision)") (TriggeredSeconds :type "Float (double-precision)") (InputAction :type "InputAction Object Reference" :default "/Game/SurvivalHorror/Input/Actions/IA_Interact.IA_Interact"))
  (bind _followcamera (`self.FollowCamera`))
  (bind _returnvalue (`SceneComponent.K2_GetComponentLocation` _followcamera))
  (:`Started`
    (bind (_outhit _returnvalue_2) (`KismetSystemLibrary.SphereTraceSingle` _returnvalue (+ (* (`SceneComponent.GetForwardVector` _followcamera) (450.0 450.0 400.0)) _returnvalue) 10.0 "TraceTypeQuery2"))
    (if _returnvalue_2
      (message `/Game/SurvivalHorror/UI/BPI_Interactable.Interact` (`.HitActor` (`GameplayStatics.BreakHitResult` _outhit)) self)
      (`self.PlayAnimMontage` "/Game/SurvivalHorror/Animations/Player/AM_Player_Pickup.AM_Player_Pickup"))))

(event `EnhancedInput|/Game/SurvivalHorror/Input/Actions/IA_Reload`
  (params (ActionValue :type Boolean) (ElapsedSeconds :type "Float (double-precision)") (TriggeredSeconds :type "Float (double-precision)") (InputAction :type "InputAction Object Reference" :default "/Game/SurvivalHorror/Input/Actions/IA_Reload.IA_Reload"))
  (bind _ammo (`self.Ammo`))
  (bind _maxammo (`self.MaxAmmo`))
  (:`Started`
    (if (and (< (`self.Ammo`) 12) (> (`self.MaxAmmo`) 0))
      (`self.PlayAnimMontage` "/Game/SurvivalHorror/Animations/Player/AM_Player_Reload.AM_Player_Reload")
      (`GameplayStatics.PlaySound2D` "/Game/SurvivalHorror/Sounds/GunReload.GunReload" 1.0 1.0 0.0 null null)
      (`KismetSystemLibrary.Delay` 0.2)
      (bind _output_get (set `self.BulletsToRecharge` (`KismetMathLibrary.Min` (- 12 _ammo) _maxammo)))
      (set `self.Ammo` (+ _output_get _ammo))
      (set `self.MaxAmmo` (- _maxammo _output_get))
      (`self.OnAmmoChanged`))))

(event `EnhancedInput|/Game/SurvivalHorror/Input/Actions/IA_Shoot`
  (params (ActionValue :type Boolean) (ElapsedSeconds :type "Float (double-precision)") (TriggeredSeconds :type "Float (double-precision)") (InputAction :type "InputAction Object Reference" :default "/Game/SurvivalHorror/Input/Actions/IA_Shoot.IA_Shoot"))
  (bind _followcamera (`self.FollowCamera`))
  (bind _returnvalue (`SceneComponent.K2_GetComponentLocation` _followcamera))
  (:`Started`
    (if (and (and (`self.bIsAiming`) (> (`self.Ammo`) 0)) (not (`self.bIsDead`)))
      (set `self.Ammo` (- (`self.Ammo`) 1))
      (`self.OnAmmoChanged`)
      (`GameplayStatics.PlaySound2D` "/Game/SurvivalHorror/Sounds/GunShooting.GunShooting" 1.0 1.0 0.0 null null)
      (`GameplayStatics.SpawnEmitterAttached` "/Game/StarterContent/Particles/P_Explosion.P_Explosion" (`self.WeaponMesh`) "None" (0.0 0.0 0.0) (struct) (0.15 0.15 0.15))
      (bind (_outhit _returnvalue_2) (`KismetSystemLibrary.LineTraceSingle` _returnvalue (+ _returnvalue (* (`SceneComponent.GetForwardVector` _followcamera) 5000.0)) "TraceTypeQuery1"))
      (if _returnvalue_2
        (`GameplayStatics.ApplyDamage` (`.HitActor` (`GameplayStatics.BreakHitResult` _outhit)) 25.0 null self)))))

(event `EnhancedInput|/Game/SurvivalHorror/Input/Actions/IA_Flashlight`
  (params (ActionValue :type Boolean) (ElapsedSeconds :type "Float (double-precision)") (TriggeredSeconds :type "Float (double-precision)") (InputAction :type "InputAction Object Reference" :default "/Game/SurvivalHorror/Input/Actions/IA_Flashlight.IA_Flashlight"))
  (:`Started`
    (`SceneComponent.ToggleVisibility` (`self.Flashlight`) false)
    (`GameplayStatics.PlaySound2D` "/Game/SurvivalHorror/Sounds/Sonido-de-Encender-o-apagar-linterna-_-Efecto-de-Sonido-Sonidos-Chingones-FX.Sonido-de-Encender-o-apagar-linterna-_-Efecto-de-Sonido-Sonidos-Chingones-FX" 1.0 1.0 0.0 null null)))

(event `EnhancedInput|/Game/SurvivalHorror/Input/Actions/IA_Crouch`
  (params (ActionValue :type Boolean) (ElapsedSeconds :type "Float (double-precision)") (TriggeredSeconds :type "Float (double-precision)") (InputAction :type "InputAction Object Reference" :default "/Game/SurvivalHorror/Input/Actions/IA_Crouch.IA_Crouch"))
  (:`Started`
    (`self.Crouch`)
    (`SceneComponent.K2_SetRelativeLocation` (`self.Mesh`) (0.0 0.0 -55.0) false false))
  (:`Completed`
    (`self.UnCrouch`)
    (`SceneComponent.K2_SetRelativeLocation` (`self.Mesh`) (0.0 0.0 -90.0) false false)))

(event `EnhancedInput|/Game/SurvivalHorror/Input/Actions/IA_Jump`
  (params (ActionValue :type Boolean) (ElapsedSeconds :type "Float (double-precision)") (TriggeredSeconds :type "Float (double-precision)") (InputAction :type "InputAction Object Reference" :default "/Game/SurvivalHorror/Input/Actions/IA_Jump.IA_Jump"))
  (:`Triggered`
    (`self.Jump`)))

(event `self.ReceiveAnyDamage`
  (params (Damage :type "Float (single-precision)") (DamageType :type "DamageType Object Reference") (InstigatedBy :type "Controller Object Reference") (DamageCauser :type "Actor Object Reference"))
  (bind _returnvalue (`GameplayStatics.GetPlayerController` 0))
  (bind _mesh (`self.Mesh`))
  (if (not (`self.bIsDead`))
    (set `self.Health` (`KismetMathLibrary.FClamp` (- (`self.Health`) Damage) 0.0 (`self.MaxHealth`)))
    (`self.OnHealthChanged`)
    (if (<= (`self.Health`) 0.0)
      (set `self.bIsDead` true)
      (`self.DisableInput` null)
      (`CharacterMovementComponent.DisableMovement` (`self.CharacterMovement`))
      (`PrimitiveComponent.SetCollisionEnabled` (`self.CapsuleComponent`) "NoCollision")
      (`PrimitiveComponent.SetCollisionProfileName` _mesh "Ragdoll" true)
      (`PrimitiveComponent.SetSimulatePhysics` _mesh true)
      (`KismetSystemLibrary.Delay` 1.0)
      (bind _returnvalue_2 (`|CreateWidget` "/Game/SurvivalHorror/UI/WBP_GameOver.WBP_GameOver_C"))
      (`UserWidget.AddToViewport` _returnvalue_2 0)
      (set `PlayerController.bShowMouseCursor` true _returnvalue)
      (`WidgetBlueprintLibrary.SetInputMode_UIOnlyEx` _returnvalue null))))

(event `EnhancedInput|/Game/SurvivalHorror/Input/Actions/IA_Pause`
  (params (ActionValue :type Boolean) (ElapsedSeconds :type "Float (double-precision)") (TriggeredSeconds :type "Float (double-precision)") (InputAction :type "InputAction Object Reference" :default "/Game/SurvivalHorror/Input/Actions/IA_Pause.IA_Pause"))
  (bind _returnvalue (`GameplayStatics.GetPlayerController` 0))
  (:`Started`
    (if (not (`self.bIsDead`))
      (bind _returnvalue_2 (`|CreateWidget` "/Game/SurvivalHorror/UI/WBP_PauseMenu.WBP_PauseMenu_C"))
      (`UserWidget.AddToViewport` _returnvalue_2 0)
      (`WidgetBlueprintLibrary.SetInputMode_UIOnlyEx` _returnvalue null)
      (set `PlayerController.bShowMouseCursor` true _returnvalue)
      (`GameplayStatics.SetGamePaused` true))))

(fn `UserConstructionScript`)