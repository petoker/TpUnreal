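; AI controller for zombie enemies that runs the BT_Zombie behavior tree on possession.
; AI Perception writes the player to the TargetActor blackboard key when successfully sensed.
; Tick also sets that key whenever the player is within a fixed range and in line of sight, independent of perception.
; Nothing here clears the key, so the controller itself never drops an acquired target.
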(event `self.ReceivePossess`
  (params (PossessedPawn :type "Pawn Object Reference"))
  (`self.RunBehaviorTree` "/Game/SurvivalHorror/Blueprints/Enemies/BT_Zombie.BT_Zombie"))

(event `self.AIPerception.OnTargetPerceptionUpdated`
  (params (Actor :type "Actor Object Reference") (Stimulus :type "AIStimulus Structure"))
  (if (and (== Actor (`GameplayStatics.GetPlayerCharacter` 0)) (`.bSuccessfullySensed` (break `AIStimulus` Stimulus)))
    (`BlackboardComponent.SetValueAsObject` (`AIBlueprintHelperLibrary.GetBlackboard` self) "TargetActor" Actor)))

(event `self.ReceiveTick`
  (params (DeltaSeconds :type "Float (single-precision)"))
  (bind _returnvalue (`self.K2_GetPawn`))
  (bind _returnvalue_2 (`GameplayStatics.GetPlayerCharacter` 0))
  (if (and (`KismetSystemLibrary.IsValid` _returnvalue) (`KismetSystemLibrary.IsValid` _returnvalue_2))
    (if (and (<= (`self.GetDistanceTo` _returnvalue _returnvalue_2) 1500.0) (`self.LineOfSightTo` _returnvalue_2))
      (`BlackboardComponent.SetValueAsObject` (`AIBlueprintHelperLibrary.GetBlackboard` self) "TargetActor" _returnvalue_2))))

(fn `UserConstructionScript`)