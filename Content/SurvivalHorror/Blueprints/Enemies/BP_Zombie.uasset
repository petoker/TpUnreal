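; BP_Zombie is a survival horror zombie enemy Blueprint that takes damage and dies into a ragdoll.
; Its AnyDamage event subtracts damage from Health while alive and sets IsDead once Health reaches zero or below, so later hits are ignored.
; Death detaches the controller, disables capsule collision and switches the mesh to the Ragdoll collision profile with physics simulation.
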(event `self.ReceiveAnyDamage`
  (params (Damage :type "Float (single-precision)") (DamageType :type "DamageType Object Reference") (InstigatedBy :type "Controller Object Reference") (DamageCauser :type "Actor Object Reference"))
  (bind _mesh (`self.Mesh`))
  (if (not (`self.bIsDead`))
    (set `self.Health` (- (`self.Health`) Damage))
    (if (<= (`self.Health`) 0.0)
      (set `self.bIsDead` true)
      (`self.DetachFromControllerPendingDestroy`)
      (`PrimitiveComponent.SetCollisionEnabled` (`self.CapsuleComponent`) "NoCollision")
      (`PrimitiveComponent.SetCollisionProfileName` _mesh "Ragdoll" true)
      (`PrimitiveComponent.SetSimulatePhysics` _mesh true))))

(fn `UserConstructionScript`)